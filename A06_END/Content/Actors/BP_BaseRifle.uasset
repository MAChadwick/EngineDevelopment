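; BP_BaseRifle is a base rifle actor that fires projectiles on behalf of the pawn it is attached to as a child actor.
; BeginPlay caches the parent actor as a Pawn, printing a warning if the cast fails.
; Attack spawns BulletClass at a skeletal mesh socket along the pawn's base aim rotation.
; Bullets take the pawn as Instigator and its AI controller as Owner.
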(event `self.ReceiveBeginPlay`
  (bind _aspawn (cast `Pawn` (`self.GetParentActor`))
    (:`then`
      (set `self.ParentPawn` _aspawn))
    (:`CastFailed`
      (`KismetSystemLibrary.PrintString` "Need to have a pawn owner"))))

(event `Attack`
  (bind _parentpawn (`self.ParentPawn`))
  (`|SpawnActorFromClass` (`self.BulletClass`) (`KismetMathLibrary.MakeTransform` (`SceneComponent.GetSocketLocation` (`self.SkeletalMesh`) (`self.SocketName`)) (`Pawn.GetBaseAimRotation` (`self.ParentPawn`))) "Undefined" "OverrideRootScale" (`AIBlueprintHelperLibrary.GetAIController` _parentpawn) _parentpawn))

(fn `UserConstructionScript`)