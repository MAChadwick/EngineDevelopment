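; BP_BaseCharacter is a base character that connects a rifle, an iron-sights animation Blueprint and a health component.
; BeginPlay spawns WeaponClass through a child actor component, validates both casts, then binds shot, attack-animation, damage and death events.
; Attacks are forwarded to the weapon, while death notifies it, plays the death animation, stops movement and disables collision.
; Both health-pickup queries return false by default.
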(event `self.ReceiveBeginPlay`
  (bind _weaponchildactorcomponent (`self.WeaponChildActorComponent`))
  ;[1 1 1] Comment
  (`ChildActorComponent.SetChildActorClass` _weaponchildactorcomponent (`self.WeaponClass`))
  (bind _asbp_base_rifle (cast `/Game/Actors/BP_BaseRifle` (`ChildActorComponent.ChildActor` _weaponchildactorcomponent))
    (:`then`
      (set `self.CurrentWeapon` _asbp_base_rifle)
      (bind _asabp_iron_sights (cast `/Game/Core/ABP_IronSights` (`SkeletalMeshComponent.GetAnimInstance` (`self.Mesh`)))
        (:`then`
          (set `self.AnimationBP` _asabp_iron_sights)
          (add `/Game/Actors/BP_BaseRifle.OnShot` (`self.CurrentWeapon`) (`|CreateDelegate` (`self.AnimationBP`) :!event `PlayAttackAnim`))
          (add `IronSightsEventGraph.OnAttackAnimationEnded` (`self.AnimationBP`) (`|CreateDelegate` (`self.CurrentWeapon`) :!event `AnimationEnded`))
          ;[1 1 1] Comment
          (add `/Game/Components/BP_HealthComponent.OnDamaged` (`self.Health`) (`|CreateDelegate` (`self.AnimationBP`) :!event `PlayHurtAnim`))
          (add `/Game/Components/BP_HealthComponent.OnDeath` (`self.Health`) (`|CreateDelegate` :!event `CharacterDeath`)))
        (:`CastFailed`
          (`KismetSystemLibrary.PrintString` "The wrong animation was set"))))
    (:`CastFailed`
      (`KismetSystemLibrary.PrintString` "We need a rifle base class"))))

(event `CharacterAttack`
  ;[1 1 1] Comment
  (`/Game/Actors/BP_BaseRifle.Attack` (`self.CurrentWeapon`)))

(event `CharacterDeath`
  (params (Percent :type "Float (double-precision)"))
  ;[1 1 1] Comment
  (`/Game/Actors/BP_BaseRifle.OwnerDied` (`self.CurrentWeapon`))
  (`IronSightsEventGraph.PlayDeathAnim` (`self.AnimationBP`) 0.0)
  (`MovementComponent.StopMovementImmediately` (`self.CharacterMovement`))
  (`self.SetActorEnableCollision` false))

(fn `CanPickupHealth`
  (returns (Yes :type Boolean))
  (return false))

(fn `ShouldPickupHealth`
  (returns (Yes :type Boolean))
  (return false))

(fn `UserConstructionScript`)