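; Base pickup actor that responds when another actor overlaps its collision box.
; The overlap passes through CanPickup and ShouldPickup checks, both returning true by default, then calls HandlePickup and HandlePostPickup.
; HandlePickup is an empty hook and HandlePostPickup destroys the actor, so child Blueprints can override the checks and effects.
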(event `self.Collision Box.OnComponentBeginOverlap`
  (params (OverlappedComponent :type "PrimitiveComponent Object Reference") (OtherActor :type "Actor Object Reference") (OtherComp :type "PrimitiveComponent Object Reference") (OtherBodyIndex :type Integer) (bFromSweep :type Boolean) (SweepResult :type "HitResult Structure (by ref)"))
  (if (`self.CanPickup` OtherActor)
    (if (`self.ShouldPickup` OtherActor)
      (`self.HandlePickup` OtherActor SweepResult)
      (`self.HandlePostPickup`))))

(event `HandlePickup`
  (params (OtherActor :type "Actor Object Reference") (SweepResult :type "HitResult Structure")))

(event `HandlePostPickup`
  (`self.K2_DestroyActor`))

(fn `CanPickup`
  (params (`Other Actor` :type "Actor Object Reference"))
  (returns (Yes :type Boolean))
  (return true))

(fn `ShouldPickup`
  (params (OtherActor :type "Actor Object Reference"))
  (returns (Yes :type Boolean))
  (return true))

(fn `UserConstructionScript`)