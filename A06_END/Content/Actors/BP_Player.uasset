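; BP_Player is the player-controlled character, handling camera look, movement and the standard attack.
; On BeginPlay it casts its controller to a PlayerController, adds WBP_HUD to the viewport and binds to the Health damaged and death events, printing a warning if the cast fails.
; Axis inputs drive controller yaw and pitch and move the pawn relative to control yaw.
; The StandardAttack press calls CharacterAttack.
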(event `self.ReceiveBeginPlay`
  (bind _health (`self.Health`))
  (`parent.ReceiveBeginPlay`)
  (bind _asplayer_controller (cast `PlayerController` (`self.GetController`))
    (:`then`
      (bind _output_get (set `self.PlayerController` _asplayer_controller))
      (bind _returnvalue (`|CreateWidget` "/Game/Core/Widgets/WBP_HUD.WBP_HUD_C" _output_get))
      (`UserWidget.AddToViewport` _returnvalue 0)
      (add `/Game/Components/BP_HealthComponent.OnDamaged` _health (`|CreateDelegate` _returnvalue :!event `SetHealth`))
      (add `/Game/Components/BP_HealthComponent.OnDeath` _health (`|CreateDelegate` _returnvalue :!event `SetHealth`)))
    (:`CastFailed`
      (`KismetSystemLibrary.PrintString` "We need a plyer controller in player"))))

(event `InputAxis|LookLeftRight`
  (params (AxisValue :type "Float (single-precision)"))
  (`self.AddControllerYawInput` AxisValue))

(event `InputAxis|LookUpDown`
  (params (AxisValue :type "Float (single-precision)"))
  (`self.AddControllerPitchInput` AxisValue))

(event `InputAxis|MoveForwardBackward`
  (params (AxisValue :type "Float (single-precision)"))
  (bind (_returnvalue_roll _returnvalue_pitch _returnvalue_yaw) (`KismetMathLibrary.BreakRotator` (`self.GetControlRotation`)))
  (`self.AddMovementInput` (`KismetMathLibrary.GetForwardVector` (`KismetMathLibrary.MakeRotator` 0.0 0.0 _returnvalue_yaw)) AxisValue))

(event `InputAxis|MoveLeftRight`
  (params (AxisValue :type "Float (single-precision)"))
  (bind (_returnvalue_roll _returnvalue_pitch _returnvalue_yaw) (`KismetMathLibrary.BreakRotator` (`self.GetControlRotation`)))
  (`self.AddMovementInput` (`KismetMathLibrary.GetRightVector` (`KismetMathLibrary.MakeRotator` 0.0 0.0 _returnvalue_yaw)) AxisValue))

(event `InputAction|StandardAttack`
  (params (Key :type "Key Structure"))
  (:`Pressed`
    (`self.CharacterAttack`)))

(fn `UserConstructionScript`
  (`parent.UserConstructionScript`))