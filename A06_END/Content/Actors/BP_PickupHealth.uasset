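; BP_PickupHealth is a health pickup actor that specializes pickup eligibility and outcome handling.
; CanPickup and ShouldPickup delegate the decision to the other actor through health-specific message calls and return its answers.
; The actor destroys itself after a pickup and plays a sound at its location when no pickup happens.
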(event `self.HandlePostPickup`
  ;[1 1 1] Comment
  (`self.K2_DestroyActor`))

(event `/Game/Actors/BP_PickupBase.HandleNoPickup`
  (`GameplayStatics.PlaySoundAtLocation` (`self.Sound`) (`self.K2_GetActorLocation`) (struct) 1.0 1.0 0.0 null null null))

(fn `CanPickup`
  (params (`Other Actor` :type "Actor Object Reference"))
  (returns (Yes :type Boolean))
  (bind _yes (message `/Game/Interfaces/BPI_Pickups.CanPickupHealth` `Other Actor`))
  (return _yes))

(fn `ShouldPickup`
  (params (OtherActor :type "Actor Object Reference"))
  (returns (Yes :type Boolean))
  (bind _yes (message `/Game/Interfaces/BPI_Pickups.ShouldPickupHealth` OtherActor))
  (return _yes))

(fn `UserConstructionScript`
  (`parent.UserConstructionScript`))